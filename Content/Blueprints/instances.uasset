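; Blueprint actor that lays out a MaxX by MaxY grid of instanced static meshes and exports the layout to testing.txt.
; The construction script adds each instance at a spacing of TileSize plus a fixed offset, prepending its location to SaveString.
; It then appends the InstancedStaticMesh display name and writes the file whenever construction runs.
; The event graph is empty, and the dynamic material and file-load nodes are unused.
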(event `self.ReceiveBeginPlay`)

(event `self.ReceiveActorBeginOverlap`
  (params (OtherActor :type "Actor Object Reference")))

(event `self.ReceiveTick`
  (params (DeltaSeconds :type "Float (single-precision)")))

(fn `UserConstructionScript`
  (bind _maxy (`self.MaxY`))
  (bind _tilesize (`self.TileSize`))
  ;[1 1 1] Make a matrix of instanced mesh objects
  (for _index (range (* (`self.MaxX`) (`self.MaxY`)))
    (bind _returnvalue (`KismetMathLibrary.MakeVector` (`KismetMathLibrary.Conv_IntToDouble` (* (+ _tilesize 260) (/ _index _maxy))) (`KismetMathLibrary.Conv_IntToDouble` (* (+ _tilesize 260) (mod _index _maxy)))))
    (`InstancedStaticMeshComponent.AddInstance` (`self.InstancedStaticMesh`) (`KismetMathLibrary.MakeTransform` _returnvalue))
    ;[1 1 1] Add all transforms to file
    (set `self.SaveString` (`KismetStringLibrary.Concat_StrStr` (`KismetStringLibrary.Conv_VectorToString` _returnvalue) (`self.SaveString`))))
  ;[1 1 1] Add mesh name to file
  (set `self.SaveString` (`KismetStringLibrary.Concat_StrStr` (`self.SaveString`) (`KismetSystemLibrary.GetDisplayName` (`self.InstancedStaticMesh`))))
  (`FileLoader.FileSaveString` (`self.SaveString`) "testing.txt"))